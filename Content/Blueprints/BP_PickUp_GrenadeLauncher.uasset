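; Grenade launcher pickup Blueprint that hands a projectile weapon to the character who picks it up.
; When the pickup component fires, it attaches the weapon to the character and, on success, sets the rifle flag on the first-person arms AnimBP.
; The construction script builds a dynamic instance of the gun material and tints it with the GunColor variable.
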(event OnPickUp(TP_PickUp)
  (params (PickUpCharacter :type Physics%20Character%20Object%20Reference))
  (bind _returnvalue (Class|PhysicsWeaponComponent|AttachWeapon (Variables|Default|GetProjectileWeapon) PickUpCharacter))
  (if _returnvalue
    (bind _asfirst_person_anim_bp (Utilities|Casting|CastToFirstPersonArms_AnimBP (Components|SkeletalMesh|GetAnimInstance (Variables|/Script/Physics.PhysicsCharacter|GetMesh1P PickUpCharacter))))
    (Variables|/Game/FirstPersonArms/Animations/FirstPersonArms_AnimBP.FirstPersonArms_AnimBP_C|SetHasRifle _asfirst_person_anim_bp true)))

(fn ConstructionScript
  (bind _returnvalue (Rendering|Material|CreateDynamicMaterialInstance (Variables|Default|GetProjectileWeapon) 0 "/Game/FPWeapon/Materials/M_FPGun.M_FPGun" "None" :!class /Script/Engine.PrimitiveComponent))
  (Rendering|Material|SetVectorParameterValue _returnvalue "Color" (Variables|Default|GetGunColor) :!class /Script/Engine.MaterialInstanceDynamic)
  (Rendering|Material|SetMaterial (Variables|Default|GetProjectileWeapon) 0 _returnvalue))