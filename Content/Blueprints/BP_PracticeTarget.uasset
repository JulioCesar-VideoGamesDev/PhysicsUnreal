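; BP_PracticeTarget is a shootable target that shatters when it takes any damage.
; It starts as a floating, gravity-free physics StaticMesh, with a GeometryCollection hidden and non-colliding.
; On AnyDamage it snaps the collection to the mesh's transform, enables its physics, collision and gravity, and hides the mesh.
; A radial impulse with high strain, scaled by damage, breaks the pieces apart.
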(event EventBeginPlay
  (bind _staticmesh (Variables|Default|GetStaticMesh))
  (bind _geometrycollection (Variables|Default|GetGeometryCollection))
  (Physics|SetSimulatePhysics _staticmesh true)
  (Physics|SetEnableGravity _staticmesh false)
  (Development|SetHiddeninGame _geometrycollection true true)
  (Collision|SetCollisionEnabled _geometrycollection "NoCollision"))

(event Collision|EventActorBeginOverlap
  (params (OtherActor :type Actor%20Object%20Reference)))

(event Game|Damage|EventAnyDamage
  (params (Damage :type Float%20%28single-precision%29) (DamageType :type Damage%20Type%20Object%20Reference) (InstigatedBy :type Controller%20Object%20Reference) (DamageCauser :type Actor%20Object%20Reference))
  (bind _geometrycollection (Variables|Default|GetGeometryCollection))
  (bind _staticmesh (Variables|Default|GetStaticMesh))
  (bind _staticmesh_2 (Variables|Default|GetStaticMesh))
  (Transformation|SetWorldLocation _geometrycollection (Transformation|GetWorldLocation _staticmesh) false true)
  (Transformation|SetWorldRotation _geometrycollection (Transformation|GetWorldRotation _staticmesh) false true)
  (Development|SetHiddeninGame _geometrycollection false true)
  (Physics|SetSimulatePhysics _geometrycollection true)
  (Physics|SetEnableGravity _geometrycollection true)
  (Collision|SetCollisionEnabled _geometrycollection "QueryAndPhysics")
  (Class|PhysicsObjectBlueprintLibrary|ApplyRadialImpulse _geometrycollection (Transformation|GetWorldLocation _geometrycollection) 1e+02 Damage "RIF_Constant" true 1e+06 true 0.0 1.0)
  (Collision|SetCollisionEnabled _staticmesh_2 "NoCollision")
  (Development|SetHiddeninGame _staticmesh_2 true false))

(fn ConstructionScript)